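; BP_FloorButton is an interactable floor button with a hieroglyph that toggles on and off and reports its state through OnPressedChanged.
; Any actor overlap enables interaction and ending a Box overlap disables it, with no check on the other actor.
; Interacted flips IsON while interaction is allowed.
; Tick recolors the hieroglyph's dynamic emissive material every frame, green when on and near-white when off.
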(event OnComponentEndOverlap(Box)
  (params (OverlappedComponent :type Primitive%20Component%20Object%20Reference) (OtherActor :type Actor%20Object%20Reference) (OtherComp :type Primitive%20Component%20Object%20Reference) (OtherBodyIndex :type Integer))
  (Variables|Default|Setinteractable false))

(event Custom|Interacted
  (if (Variables|Default|Getinteractable)
    (bind _output_get (Variables|Default|SetisON (not (Variables|Default|GetisON))))
    (Default|CallOnPressedChanged _output_get)))

(event EventBeginPlay
  (bind _returnvalue (Rendering|Material|CreateDynamicMaterialInstance (Variables|Default|GetSM_hieroglyph_007) 0 "/Game/LowPolyAssets/Materials/MI_Emission.MI_Emission" "None" :!class /Script/Engine.PrimitiveComponent))
  (Variables|Default|SetHyeroglyphMat _returnvalue))

(event EventTick
  (params (DeltaSeconds :type Float%20%28single-precision%29))
  (bind _hyeroglyphmat (Variables|Default|GetHyeroglyphMat))
  (if (Variables|Default|GetisON)
    (Rendering|Material|SetVectorParameterValue _hyeroglyphmat "ButtonColor" "(R=0.000000,G=1.000000,B=0.161700,A=1.000000)" :!class /Script/Engine.MaterialInstanceDynamic)
    (else
      (Rendering|Material|SetVectorParameterValue _hyeroglyphmat "ButtonColor" "(R=1.000000,G=0.965388,B=0.960119,A=1.000000)" :!class /Script/Engine.MaterialInstanceDynamic))))

(event Collision|EventActorBeginOverlap
  (params (OtherActor :type Actor%20Object%20Reference))
  (Variables|Default|Setinteractable true))

(fn ConstructionScript)