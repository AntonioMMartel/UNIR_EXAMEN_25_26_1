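; Double sliding door actor that opens and closes as the referenced button's pressed state changes.
; It binds to that button on BeginPlay and runs a separate open or close timeline, each always played from start.
; The timelines move the two leaves in opposite directions along world X or Y, chosen by DoorOrientedRight, using hardcoded offsets from the actor's location.
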(event Custom|OpenDoor
  (bind _returnvalue (Transformation|GetActorTransform))
  (bind _returnvalue_2 (Transformation|GetActorTransform))
  (bind (_location _rotation _scale) (Math|Transform|BreakTransform _returnvalue))
  (bind (_location_2 _rotation_2 _scale_2) (Math|Transform|BreakTransform _returnvalue_2))
  (bind _alpha (Timeline|TM_DoorOpen PlayFromStart)
    (:Update
      (Transformation|SetWorldTransform (Variables|Default|GetSM_door_left) (Math|Transform|MakeTransform (+ (+ _location (Math|Vector|SelectVector "-50.000000,0.000000,0.000000" "0.000000,-50.000000,0.000000" (Variables|Default|GetDoorOrientedRight))) (* _alpha (select (Variables|Default|GetDoorOrientedRight) "-100.000000,0.000000,0.000000" "0.000000,-100.000000,0.000000"))) _rotation _scale) false false)
      (Transformation|SetWorldTransform (Variables|Default|GetSM_door_right) (Math|Transform|MakeTransform (+ (+ _location_2 (Math|Vector|SelectVector "50.000000,0.000000,0.000000" "0.000000,50.000000,0.000000" (Variables|Default|GetDoorOrientedRight))) (* (* _alpha (select (Variables|Default|GetDoorOrientedRight) "-100.000000,0.000000,0.000000" "0.000000,-100.000000,0.000000")) -1.0)) _rotation_2 _scale_2) false false))))

(event Custom|ButtonChanged
  (params (ButtonState :type Boolean))
  (if ButtonState
    (CallFunction|OpenDoor)
    (else
      (CallFunction|CloseDoor))))

(event Custom|CloseDoor
  (bind _returnvalue (Transformation|GetActorTransform))
  (bind _returnvalue_2 (Transformation|GetActorTransform))
  (bind (_location _rotation _scale) (Math|Transform|BreakTransform _returnvalue))
  (bind (_location_2 _rotation_2 _scale_2) (Math|Transform|BreakTransform _returnvalue_2))
  (bind _alpha (Timeline|Timeline PlayFromStart)
    (:Update
      (Transformation|SetWorldTransform (Variables|Default|GetSM_door_left) (Math|Transform|MakeTransform (+ (+ _location_2 (Math|Vector|SelectVector "-150.000000,0.000000,0.000000" "0.000000,-150.000000,0.000000" (Variables|Default|GetDoorOrientedRight))) (* _alpha (select (Variables|Default|GetDoorOrientedRight) "-100.000000,0.000000,0.000000" "0.000000,-100.000000,0.000000"))) _rotation_2 _scale_2) false false)
      (Transformation|SetWorldTransform (Variables|Default|GetSM_door_right) (Math|Transform|MakeTransform (+ (+ _location (Math|Vector|SelectVector "150.000000,0.000000,0.000000" "0.000000,150.000000,0.000000" (Variables|Default|GetDoorOrientedRight))) (* (* _alpha (select (Variables|Default|GetDoorOrientedRight) "-100.000000,0.000000,0.000000" "0.000000,-100.000000,0.000000")) -1.0)) _rotation _scale) false false))))

(event EventBeginPlay
  (EventDispatchers|AssignOnPressedChanged (Variables|Default|GetButtonReference) (delegate Custom|ButtonChanged)))

(fn ConstructionScript)